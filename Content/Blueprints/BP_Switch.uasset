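; BP_Switch is a switch actor with a button component that moves while something overlaps its Box trigger.
; Box begin and end overlap toggle IsTracking, which makes Tick lower the button's relative X by a fixed per-frame step, clamped between zero and ButtonOffset.
; Whenever the clamped position equals ButtonOffset during tracking, Tick calls ButtonSwitch, which only prints a placeholder message.
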(event OnComponentBeginOverlap(Box)
  (params (OverlappedComponent :type Primitive%20Component%20Object%20Reference) (OtherActor :type Actor%20Object%20Reference) (OtherComp :type Primitive%20Component%20Object%20Reference) (OtherBodyIndex :type Integer) (bFromSweep :type Boolean) (SweepResult :type Hit%20Result%20Structure%20%28by%20ref%29))
  (Variables|Default|SetisTracking true))

(event OnComponentEndOverlap(Box)
  (params (OverlappedComponent :type Primitive%20Component%20Object%20Reference) (OtherActor :type Actor%20Object%20Reference) (OtherComp :type Primitive%20Component%20Object%20Reference) (OtherBodyIndex :type Integer))
  (Variables|Default|SetisTracking false))

(event Custom|Button%20Switch
  (Development|PrintString "Hello"))

(event EventTick
  (params (DeltaSeconds :type Float%20%28single-precision%29))
  (bind _button (Variables|Default|GetButton))
  (if (Variables|Default|GetisTracking)
    (bind _output_get (Variables|Default|SetCurrent_Offset (Math|Float|Clamp(Float) (- (.x (Variables|/Script/Engine.SceneComponent|GetRelativeLocation _button)) 0.5) 0.0 (Variables|Default|GetButton_Offset))))
    (Transformation|SetRelativeLocation _button (Math|Vector|MakeVector _output_get 0.0 0.0) false false)
    (if (== (Variables|Default|GetCurrent_Offset) (Variables|Default|GetButton_Offset))
      (CallFunction|ButtonSwitch))))

(fn ConstructionScript)