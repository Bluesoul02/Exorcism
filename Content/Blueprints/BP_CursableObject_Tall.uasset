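; BP_CursableObject_Tall is a cursed world object that is cleansed by keeping a BP_Cross inside its capsule.
; Overlap enables Tick, which billboards a WBP_Cleansing progress widget to the camera and accumulates time.
; Leaving early disables Tick and resets progress, though the widget is still set visible.
; At the required time it plays particles and sound, destroys the curse components and fires OnObjectCleansed.
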(event OnComponentBeginOverlap(Capsule)
  (params (OverlappedComponent :type Primitive%20Component%20Object%20Reference) (OtherActor :type Actor%20Object%20Reference) (OtherComp :type Primitive%20Component%20Object%20Reference) (OtherBodyIndex :type Integer) (bFromSweep :type Boolean) (SweepResult :type Hit%20Result%20Structure%20%28by%20ref%29))
  (if (Variables|Default|GetIsCursed)
    (Utilities|Casting|CastToBP_Cross OtherActor)
    (Actor|Tick|SetActorTickEnabled true)
    (Rendering|SetVisibility (Variables|Default|GetWidget) true false)))

(event OnComponentEndOverlap(Capsule)
  (params (OverlappedComponent :type Primitive%20Component%20Object%20Reference) (OtherActor :type Actor%20Object%20Reference) (OtherComp :type Primitive%20Component%20Object%20Reference) (OtherBodyIndex :type Integer))
  (bind _widget (Variables|Default|GetWidget))
  (if (Variables|Default|GetIsCursed)
    (Utilities|Casting|CastToBP_Cross OtherActor)
    (Actor|Tick|SetActorTickEnabled false)
    (Variables|Default|SetCleansingTimeDone 0.0)
    (Utilities|IsValid _widget
      (:Is%20Valid
        (bind _aswbp_cleansing (Utilities|Casting|CastToWBP_Cleansing (UserInterface|GetUserWidgetObject _widget)))
        (Variables|/Game/UI/WBP_Cleansing.WBP_Cleansing_C|SetCleansingProgress _aswbp_cleansing 0.0)
        (Rendering|SetVisibility _widget true false)))))

(event EventBeginPlay)

(event Collision|EventActorBeginOverlap
  (params (OtherActor :type Actor%20Object%20Reference)))

(event EventTick
  (params (DeltaSeconds :type Float%20%28single-precision%29))
  (bind _widget (Variables|Default|GetWidget))
  (Transformation|SetWorldRotation _widget (Math|Rotator|FindLookatRotation (Transformation|GetWorldLocation _widget) (Transformation|GetActorLocation (Game|GetPlayerCameraManager 0))) false false)
  (bind _output_get (Variables|Default|SetCleansingTimeDone (+ DeltaSeconds (Variables|Default|GetCleansingTimeDone))))
  (bind _aswbp_cleansing (Utilities|Casting|CastToWBP_Cleansing (UserInterface|GetUserWidgetObject _widget)))
  (Variables|/Game/UI/WBP_Cleansing.WBP_Cleansing_C|SetCleansingProgress _aswbp_cleansing _output_get)
  (if (>= _output_get (Variables|Default|GetCleansingTimeNeeded))
    (Utilities|FlowControl|Sequence
      (:then_0
        (AddComponent|AddParticleSystemComponent false))
      (:then_1
        (Audio|PlaySoundatLocation "/Game/SFX/Cleanse.Cleanse" (Transformation|GetActorLocation) "0, 0, 0" 0.4 1.0 0.0 "/Game/SFX/Ghost/DefaultSoundAttenuation.DefaultSoundAttenuation" 0 0 0))
      (:then_2
        (CallFunction|RemoveCurse)
        (Actor|Tick|SetActorTickEnabled false)
        (Default|CallOnObjectCleansed)))))

(fn ConstructionScript
  (Components|StaticMesh|SetStaticMesh (Variables|Default|GetVariableMesh) (Variables|Default|GetParentMesh)))

(fn RemoveCurse
  (Variables|Default|SetIsCursed false)
  (Components|DestroyComponent (Variables|Default|GetP_Monster_Death_Small))
  (Components|DestroyComponent (Variables|Default|GetWidget))
  (Components|DestroyComponent (Variables|Default|GetCapsule)))