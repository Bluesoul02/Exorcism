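; BP_Holster is a holster actor that stores a single player item.
; When a BP_Player_Items actor overlaps HolsterMesh while the holster is empty, it records the item, flags its GrabComponent as holstered and passes it a reference to itself.
; It then teleports the item to the mesh, attaches it with the socket name "Holster" and sets HasItem.
; This Blueprint contains no release logic.
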(event OnComponentBeginOverlap(HolsterMesh)
  (params (OverlappedComponent :type Primitive%20Component%20Object%20Reference) (OtherActor :type Actor%20Object%20Reference) (OtherComp :type Primitive%20Component%20Object%20Reference) (OtherBodyIndex :type Integer) (bFromSweep :type Boolean) (SweepResult :type Hit%20Result%20Structure%20%28by%20ref%29))
  (bind _asbp_player_items (Utilities|Casting|CastToBP_Player_Items OtherActor))
  (if (not (Variables|Default|GethasItem))
    (bind _output_get (Variables|Default|SetHolsteredItem _asbp_player_items))
    (Variables|/Game/VRTemplate/Blueprints/GrabComponent.GrabComponent_C|SetisHolstered (Actor|GetComponentbyClass _output_get "/Game/VRTemplate/Blueprints/GrabComponent.GrabComponent_C") true)
    (Variables|/Game/VRTemplate/Blueprints/GrabComponent.GrabComponent_C|SetHolster (Actor|GetComponentbyClass _output_get "/Game/VRTemplate/Blueprints/GrabComponent.GrabComponent_C") self)
    (Transformation|SetActorLocation (Variables|Default|GetHolsteredItem) (Transformation|GetWorldLocation (Variables|Default|GetHolsterMesh)) false true)
    (Transformation|AttachActorToActor (Variables|Default|GetHolsteredItem) self "Holster" "SnapToTarget" "SnapToTarget" "KeepRelative" true)
    (Variables|Default|SethasItem true)))

(event EventBeginPlay)

(event Collision|EventActorBeginOverlap
  (params (OtherActor :type Actor%20Object%20Reference)))

(event EventTick
  (params (DeltaSeconds :type Float%20%28single-precision%29)))

(fn ConstructionScript)