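; Small cursable physics prop that is cleansed by keeping a BP_Cross inside its trigger sphere.
; While cursed, physics is off; cross overlap enables Tick, which accumulates time into a camera-facing progress widget, and leaving resets it.
; At the required time it plays particle and sound effects, removes the curse components, changes the grab type, enables physics and broadcasts OnObjectCleansed.
; The construction script applies ParentMesh to the mesh component.
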(event OnComponentBeginOverlap(Sphere)
  (params (OverlappedComponent :type Primitive%20Component%20Object%20Reference) (OtherActor :type Actor%20Object%20Reference) (OtherComp :type Primitive%20Component%20Object%20Reference) (OtherBodyIndex :type Integer) (bFromSweep :type Boolean) (SweepResult :type Hit%20Result%20Structure%20%28by%20ref%29))
  (if (Variables|Default|GetIsCursed)
    (Utilities|Casting|CastToBP_Cross OtherActor)
    (Actor|Tick|SetActorTickEnabled true)
    (Rendering|SetVisibility (Variables|Default|GetWidget) true false)))

(event OnComponentEndOverlap(Sphere)
  (params (OverlappedComponent :type Primitive%20Component%20Object%20Reference) (OtherActor :type Actor%20Object%20Reference) (OtherComp :type Primitive%20Component%20Object%20Reference) (OtherBodyIndex :type Integer))
  (bind _widget (Variables|Default|GetWidget))
  (if (Variables|Default|GetIsCursed)
    (Utilities|Casting|CastToBP_Cross OtherActor)
    (Actor|Tick|SetActorTickEnabled false)
    (Variables|Default|SetCleansingTimeDone 0.0)
    (Utilities|IsValid _widget
      (:Is%20Valid
        (bind _aswbp_cleansing (Utilities|Casting|CastToWBP_Cleansing (UserInterface|GetUserWidgetObject _widget)))
        (Variables|/Game/UI/WBP_Cleansing.WBP_Cleansing_C|SetCleansingProgress _aswbp_cleansing 0.0)
        (Rendering|SetVisibility _widget true false)))))

(event EventBeginPlay
  (if (Variables|Default|GetIsCursed)
    (bind _asprimitive_component (Utilities|Casting|CastToPrimitiveComponent (Transformation|GetAttachParent (Variables|Default|GetGrabComponent))))
    (Physics|SetSimulatePhysics _asprimitive_component false)
    (else
      (bind _asprimitive_component_2 (Utilities|Casting|CastToPrimitiveComponent (Transformation|GetAttachParent (Variables|Default|GetGrabComponent))))
      (Physics|SetSimulatePhysics _asprimitive_component_2 true))))

(event EventTick
  (params (DeltaSeconds :type Float%20%28single-precision%29))
  (bind _widget (Variables|Default|GetWidget))
  (Transformation|SetWorldRotation _widget (Math|Rotator|FindLookatRotation (Transformation|GetWorldLocation _widget) (Transformation|GetActorLocation (Game|GetPlayerCameraManager 0))) false false)
  (bind _output_get (Variables|Default|SetCleansingTimeDone (+ DeltaSeconds (Variables|Default|GetCleansingTimeDone))))
  (bind _aswbp_cleansing (Utilities|Casting|CastToWBP_Cleansing (UserInterface|GetUserWidgetObject _widget)))
  (Variables|/Game/UI/WBP_Cleansing.WBP_Cleansing_C|SetCleansingProgress _aswbp_cleansing _output_get)
  (if (>= _output_get (Variables|Default|GetCleansingTimeNeeded))
    (Utilities|FlowControl|Sequence
      (:then_0
        (AddComponent|AddParticleSystemComponent false))
      (:then_1
        (Audio|PlaySoundatLocation "/Game/SFX/Cleanse.Cleanse" (Transformation|GetActorLocation) "0, 0, 0" 0.4 1.0 0.0 (Variables|/Script/Engine.AudioComponent|GetAttenuationSettings (Variables|Default|GetAudio)) 0 0 0))
      (:then_2
        (CallFunction|RemoveCurse)
        (Actor|Tick|SetActorTickEnabled false)
        (Default|CallOnObjectCleansed)))))

(fn ConstructionScript
  (Components|StaticMesh|SetStaticMesh (Variables|Default|GetVariableMesh) (Variables|Default|GetParentMesh)))

(fn RemoveCurse
  (Variables|Default|SetIsCursed false)
  (Components|DestroyComponent (Variables|Default|GetP_Monster_Death_Small))
  (Components|DestroyComponent (Variables|Default|GetWidget))
  (Components|DestroyComponent (Variables|Default|GetAudio))
  (Components|DestroyComponent (Variables|Default|GetSphere))
  (Variables|/Game/VRTemplate/Blueprints/GrabComponent.GrabComponent_C|SetGrabType (Variables|Default|GetGrabComponent) "NewEnumerator4")
  (Physics|SetSimulatePhysics (Variables|Default|GetVariableMesh) true))