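; BP_Cross is a VR cross that the player charges with the trigger to cleanse ghosts.
; While the trigger is held, Tick accumulates charge time, disables the VRPawn's movement and feeds the charge to the WBP_Cross widget.
; Release hides the widget, restores walking and resets the charge.
; If fully charged, it also line-traces forward from Aim, with debug drawing, and calls CleanseGhost on a hit BP_Ghost whose mesh is visible.
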(event EventBeginPlay)

(event Collision|EventActorBeginOverlap
  (params (OtherActor :type Actor%20Object%20Reference)))

(event EventTick
  (params (DeltaSeconds :type Float%20%28single-precision%29))
  (if (Variables|Default|GetbIsFiring)
    (Variables|Default|SetLoading (+ (Variables|Default|GetLoading) DeltaSeconds))
    (bind _asvrpawn (Utilities|Casting|CastToVRPawn (Game|Player|GetPlayerPawn 0)))
    (Pawn|Components|CharacterMovement|DisableMovement (Variables|/Script/Engine.Character|GetCharacterMovement _asvrpawn))
    (bind _aswbp_cross (Utilities|Casting|CastToWBP_Cross (UserInterface|GetUserWidgetObject (Variables|Default|GetWidget))))
    (Variables|/Game/UI/WBP_Cross.WBP_Cross_C|SetLoading _aswbp_cross (Variables|Default|GetLoading))))

(event EventTriggerPressed
  (Variables|Default|SetbIsFiring true)
  (Rendering|SetVisibility (Variables|Default|GetWidget) true false))

(event EventTriggerReleased
  (bind _widget (Variables|Default|GetWidget))
  (bind _aim (Variables|Default|Getaim))
  (bind _returnvalue (Transformation|GetWorldLocation _aim))
  (bind _returnvalue_2 (Transformation|GetWorldRotation _aim))
  (Variables|Default|SetbIsFiring false)
  (Rendering|SetVisibility _widget false false)
  (bind _aswbp_cross (Utilities|Casting|CastToWBP_Cross (UserInterface|GetUserWidgetObject _widget)))
  (Variables|/Game/UI/WBP_Cross.WBP_Cross_C|SetLoading _aswbp_cross 0.0)
  (bind _asvrpawn (Utilities|Casting|CastToVRPawn (Game|Player|GetPlayerPawn 0)))
  (Pawn|Components|CharacterMovement|SetMovementMode (Variables|/Script/Engine.Character|GetCharacterMovement _asvrpawn) "MOVE_Walking" 0)
  (if (>= (Variables|Default|GetLoading) (Variables|Default|GetLoading%20time))
    (bind _outhit (Collision|LineTraceByChannel _returnvalue (+ (* (Math|Vector|GetForwardVector (Math|Rotator|MakeRotator (.roll _returnvalue_2) (.pitch _returnvalue_2) (.yaw _returnvalue_2))) 1.5e+03) _returnvalue) "TraceTypeQuery1" false 0 "ForDuration" true "(R=1.000000,G=0.000000,B=0.000000,A=1.000000)" "(R=0.000000,G=1.000000,B=0.000000,A=1.000000)" 1.0))
    (bind _asbp_ghost (Utilities|Casting|CastToBP_Ghost (.HitActor (Collision|BreakHitResult _outhit)))
      (:then
        (if (Rendering|IsVisible (Variables|/Script/Engine.Character|GetMesh _asbp_ghost))
          (Default|CleanseGhost _asbp_ghost)))
      (:CastFailed
        _))
    (Variables|Default|SetLoading 0.0)
    (else
      (Variables|Default|SetLoading 0.0))))

(fn ConstructionScript)