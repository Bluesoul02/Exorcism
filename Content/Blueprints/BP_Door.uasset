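; BP_Door is a physics-driven door that the player swings open by grabbing it in VR.
; On grab, it picks the VRPawn's left or right hand from the controller's motion source and enables Tick; release clears the state and disables it.
; Each tick applies torque from the cross product of the hand's current and previous world locations, scaled by a multiplier and optionally negated.
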(event OnDropped(GrabComponent)
  (Variables|Default|SetHand 0)
  (Variables|Default|SetOldHandLocation "0, 0, 0")
  (Variables|Default|SetTorque "0, 0, 0")
  (Actor|Tick|SetActorTickEnabled false))

(event OnGrabbed(GrabComponent)
  (if (Utilities|Name|Equal(Name) (Variables|/Script/HeadMountedDisplay.MotionControllerComponent|GetMotionSource (Variables|/Game/VRTemplate/Blueprints/GrabComponent.GrabComponent_C|GetMotionControllerRef (Variables|Default|GetGrabComponent))) "Left")
    (bind _output_get (Variables|Default|SetHand (Variables|Default|GetLeftHand)))
    (Variables|Default|SetOldHandLocation (Transformation|GetWorldLocation _output_get))
    (Actor|Tick|SetActorTickEnabled true)
    (else
      (bind _output_get_2 (Variables|Default|SetHand (Variables|Default|GetRightHand)))
      (Variables|Default|SetOldHandLocation (Transformation|GetWorldLocation _output_get_2))
      (Actor|Tick|SetActorTickEnabled true))))

(event EventBeginPlay
  (bind _asvrpawn (Utilities|Casting|CastToVRPawn (Game|Player|GetPlayerPawn 0)))
  (Variables|Default|SetRightHand (Variables|/Game/VRTemplate/Blueprints/VRPawn.VRPawn_C|GetRightHand _asvrpawn))
  (Variables|Default|SetLeftHand (Variables|/Game/VRTemplate/Blueprints/VRPawn.VRPawn_C|GetLeftHand _asvrpawn)))

(event EventTick
  (params (DeltaSeconds :type Float%20%28single-precision%29))
  (bind _hand (Variables|Default|GetHand))
  (bind _returnvalue (Transformation|GetWorldLocation _hand))
  (Utilities|IsValid (Variables|Default|GetHand)
    (:Is%20Valid
      (if (not (Math|Vector|VectorIsZero (Variables|Default|GetOldHandLocation)))
        ;[1 1 1] Open door with torque (using physics)
        (if (Variables|Default|GetUseNegate)
          (Variables|Default|SetTorque (Math|Vector|NegateVector (* (Math|Vector|CrossProduct _returnvalue (Variables|Default|GetOldHandLocation)) (Variables|Default|GetRotationSpeedMultiplicator))))
          (else
            (Variables|Default|SetTorque (* (Math|Vector|CrossProduct _returnvalue (Variables|Default|GetOldHandLocation)) (Variables|Default|GetRotationSpeedMultiplicator)))))
        (Class|PrimitiveComponent|AddTorqueinDegrees (Variables|Default|GetDoor) (Variables|Default|GetTorque) "None" true)
        (Variables|Default|SetOldHandLocation _returnvalue)))))

(fn ConstructionScript)